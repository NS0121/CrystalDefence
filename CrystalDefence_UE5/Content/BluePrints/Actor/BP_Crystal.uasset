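; BP_Crystal is a crystal actor that supplies MP to the player while it exists and can be broken by enemies.
; Every Tick it adds a fixed MP amount through MyGameInstance, without delta-time scaling.
; When a component tagged EnemyB overlaps its Sphere, it waits briefly, plays a break sound and spawns a Geometry Collection replacement at the mesh transform.
; It then notifies VRGameMode of the break and destroys itself.
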(event OnComponentBeginOverlap(Sphere)
  (params (OverlappedComponent :type Primitive%20Component%20Object%20Reference) (OtherActor :type Actor%20Object%20Reference) (OtherComp :type Primitive%20Component%20Object%20Reference) (OtherBodyIndex :type Integer) (bFromSweep :type Boolean) (SweepResult :type Hit%20Result%20Structure%20%28by%20ref%29))
  (if (Components|ComponentHasTag OtherComp "EnemyB")
    (Utilities|FlowControl|Delay 0.5)
    (Audio|PlaySoundatLocation "/Game/Sound/SE_CrystalBreak.SE_CrystalBreak" (Transformation|GetActorLocation self) "0, 0, 0" 1.0 1.0 0.0 0 0 0)
    (Game|SpawnActorfromClass "/Game/Meshes/SphereBrush_G/BP_PedestalCrystal_GeometryCollection.BP_PedestalCrystal_GeometryCollection_C" (Transformation|GetWorldTransform (Variables|Default|GetStaticMesh)) "Undefined" 0 0)
    (bind _asvrgame_mode (Utilities|Casting|CastToVRGameMode (Game|GetGameMode)))
    (Default|FNCCrystalBreak _asvrgame_mode)
    (Actor|DestroyActor)))

(event EventBeginPlay)

(event Collision|EventActorBeginOverlap
  (params (OtherActor :type Actor%20Object%20Reference)))

(event EventTick
  (params (DeltaSeconds :type Float%20%28single-precision%29))
  (bind _asmy_game_instance (Utilities|Casting|CastToMyGameInstance (Game|GetGameInstance)))
  (Default|PlusMP _asmy_game_instance 1e+01))

(fn ConstructionScript)