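; BP_Barrier is a destructible barrier actor that loses HP when components tagged EnemyB overlap its sphere.
; Each hit creates a dynamic material on Sphere1, sets the impact position, then runs timelines animating a ripple radius followed by opacity.
; Non-lethal hits play a hit sound.
; The lethal hit briefly delays, plays a break sound, spawns a shield Geometry Collection at a hardcoded transform and destroys the actor.
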(event OnComponentBeginOverlap(Sphere)
  (params (OverlappedComponent :type Primitive%20Component%20Object%20Reference) (OtherActor :type Actor%20Object%20Reference) (OtherComp :type Primitive%20Component%20Object%20Reference) (OtherBodyIndex :type Integer) (bFromSweep :type Boolean) (SweepResult :type Hit%20Result%20Structure%20%28by%20ref%29))
  (if (Components|ComponentHasTag OtherComp "EnemyB")
    (Utilities|FlowControl|Sequence
      (:then_0
        (bind _returnvalue (Rendering|Material|CreateDynamicMaterialInstance (Variables|Default|GetSphere1) 0 0 "None" :!class /Script/Engine.PrimitiveComponent))
        (Rendering|Material|SetVectorParameterValue _returnvalue "Pos" (Math|Conversions|ToLinearColor(Vector) (Transformation|GetWorldLocation OtherComp)) :!class /Script/Engine.MaterialInstanceDynamic)
        (Rendering|Material|SetScalarParameterValue _returnvalue "Opacity" 0.8 :!class /Script/Engine.MaterialInstanceDynamic)
        (bind _newtrack_0 (Timeline|RadiusAnim PlayFromStart)
          (:Update
            (Rendering|Material|SetScalarParameterValue _returnvalue "Radius" (* _newtrack_0 2e+02) :!class /Script/Engine.MaterialInstanceDynamic))
          (:Finished
            (bind _newtrack_0_2 (Timeline|OpacityAnim PlayFromStart)
              (:Update
                (Rendering|Material|SetScalarParameterValue _returnvalue "Opacity" _newtrack_0_2 :!class /Script/Engine.MaterialInstanceDynamic))))))
      (:then_1
        (if (<= (- (Variables|Default|GetHP) 1e+01) 0.0)
          (Utilities|FlowControl|DoOnce false
            (:Completed
              (Utilities|FlowControl|Delay 0.5)
              (Audio|PlaySoundatLocation "/Game/Sound/SE_BarrierBreak.SE_BarrierBreak" (Transformation|GetActorLocation self) "0, 0, 0" 1.0 1.0 0.0 "/Game/Sound/SlimeSoundAttenuation.SlimeSoundAttenuation" 0 0)
              (Game|SpawnActorfromClass "/Game/Meshes/BP_Shield_Box_GeometryCollection.BP_Shield_Box_GeometryCollection_C" (Math|Transform|MakeTransform "-1760.000000, 0,140.000000" "0,-90.000000, 0" "1,1,1") "Undefined" 0 0)
              (Actor|DestroyActor)))
          (else
            (Variables|Default|SetHP (- (Variables|Default|GetHP) 1e+01))
            (Audio|PlaySoundatLocation "/Game/Sound/SE_Barrier.SE_Barrier" (Transformation|GetActorLocation self) "0, 0, 0" 0.3 1.0 0.0 "/Game/Sound/SlimeSoundAttenuation.SlimeSoundAttenuation" 0 0)))))))

(fn ConstructionScript)