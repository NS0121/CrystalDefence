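; Temporary turret that targets the nearest "Enemy"-tagged actor in range, then despawns with a particle burst after a minute.
; Tick keeps that target until invalid, aiming at it while a quadratically growing roll spins up the barrels.
; Past a spin threshold it spawns three BP_NormalBullet actors every targeting frame, since the spin never resets.
; The line trace and printout are debug-only; FNC_Shot is empty.
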(event EventBeginPlay
  (Utilities|FlowControl|Delay 6e+01)
  (Effects|SpawnEmitteratLocation "/Game/InfinityBladeEffects/Effects/FX_Skill_Leap/P_Skill_Leap_Base_Charge_Weapon.P_Skill_Leap_Base_Charge_Weapon" (Transformation|GetActorLocation self) "0, 0, 0" "5.000000,5.000000,5.000000")
  (Actor|DestroyActor))

(event Collision|EventActorBeginOverlap
  (params (OtherActor :type Actor%20Object%20Reference)))

(event EventTick
  (params (DeltaSeconds :type Float%20%28single-precision%29))
  (bind _scene5 (Variables|Default|GetScene5))
  (bind _scene4 (Variables|Default|GetScene4))
  (bind _returnvalue (Transformation|GetWorldLocation _scene4))
  (bind _returnvalue_2 (Transformation|GetSocketTransform _scene5 "None" "RTS_World"))
  (Variables|Default|SetDeltaSec DeltaSeconds)
  (Utilities|IsValid (Variables|Default|GetNewVar_0)
    (:Is%20Valid
      (Utilities|FlowControl|Sequence
        (:then_0
          (Transformation|SetWorldRotation (Variables|Default|GetScene5) (Math|Rotator|FindLookatRotation _returnvalue (Transformation|GetActorLocation (Variables|Default|GetNewVar_0))) false false)
          (Collision|LineTraceByChannel _returnvalue (Transformation|GetActorLocation (Variables|Default|GetNewVar_0)) "TraceTypeQuery1" false 0 "ForOneFrame")
          (bind _output_get (Variables|Default|SetRotation (+ (Variables|Default|GetDeltaSec) (Variables|Default|GetRotation))))
          (Transformation|SetRelativeRotation (Variables|Default|GetScene5) (Math|Rotator|MakeRotator (* _output_get (Variables|Default|GetRotation) 2e+01) (.pitch (.rotation _returnvalue_2)) (.yaw (.rotation _returnvalue_2))) false false)
          (Development|PrintString (Utilities|String|ToString(Float) (* _output_get (Variables|Default|GetRotation) 2e+01)) true true "(R=0.000000,G=0.660000,B=1.000000,A=1.000000)" 0.1)
          (if (>= (* _output_get (Variables|Default|GetRotation) 2e+01) 1e+04)
            (Game|SpawnActorfromClass "/Game/BluePrints/Bullet/NormalBullet/BP_NormalBullet.BP_NormalBullet_C" (Transformation|GetWorldTransform (Variables|Default|GetScene1)) "Undefined" 0 0)
            (Game|SpawnActorfromClass "/Game/BluePrints/Bullet/NormalBullet/BP_NormalBullet.BP_NormalBullet_C" (Transformation|GetWorldTransform (Variables|Default|GetScene)) "Undefined" 0 0)
            (Game|SpawnActorfromClass "/Game/BluePrints/Bullet/NormalBullet/BP_NormalBullet.BP_NormalBullet_C" (Transformation|GetWorldTransform (Variables|Default|GetScene3)) "Undefined" 0 0)))))
    (:Is%20Not%20Valid
      (Variables|Default|SetMinDistance 1e+04)
      (bind _outactors (Actor|GetAllActorswithTag "Enemy"))
      (for _array_element _outactors
        (if (< (Transformation|GetDistanceTo _array_element self) (Variables|Default|GetMinDistance))
          (Variables|Default|SetMinDistance (Transformation|GetDistanceTo _array_element self))
          (Variables|Default|SetNewVar_0 _array_element))))))

(fn ConstructionScript)

(fn FNCShot)