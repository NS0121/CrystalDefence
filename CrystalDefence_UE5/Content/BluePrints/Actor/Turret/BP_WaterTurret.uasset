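; Water turret actor that attacks FireEnemy-tagged actors and removes itself after a fixed lifetime.
; Tick takes the first tagged actor as target, turns Center toward it and starts a timeline once per acquisition.
; The timeline spins the magic circle and its Shot event spawns a water explosion with sound at the target's XY near ground height.
; On expiry it plays a particle effect and decrements the GameInstance turret count.
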(event EventBeginPlay
  (Utilities|FlowControl|Delay 2e+01)
  (Effects|SpawnEmitteratLocation "/Game/InfinityBladeEffects/Effects/FX_Skill_Leap/P_Skill_Leap_Base_Charge_Weapon.P_Skill_Leap_Base_Charge_Weapon" (Transformation|GetWorldLocation (Variables|Default|GetCenter)) "0, 0, 0" "2.000000,2.000000,2.000000")
  (bind _asmy_game_instance (Utilities|Casting|CastToMyGameInstance (Game|GetGameInstance)))
  (Variables|/Game/BluePrints/MyGameInstance.MyGameInstance_C|SetTurret _asmy_game_instance (- (Variables|/Game/BluePrints/MyGameInstance.MyGameInstance_C|GetTurret _asmy_game_instance) 1))
  (Actor|DestroyActor))

(event Collision|EventActorBeginOverlap
  (params (OtherActor :type Actor%20Object%20Reference)))

(event EventTick
  (params (DeltaSeconds :type Float%20%28single-precision%29))
  (bind _center (Variables|Default|GetCenter))
  (Utilities|IsValid (Variables|Default|GetTarget)
    (:Is%20Valid
      (Transformation|SetRelativeRotation _center (Math|Rotator|FindLookatRotation (Transformation|GetWorldLocation _center) (Transformation|GetActorLocation (Variables|Default|GetTarget))) false false)
      (Utilities|FlowControl|DoOnce false :!label _label
        (:Completed
          (bind _rotaion (Timeline|TL_Rotation PlayFromStart)
            (:Update
              (Transformation|SetRelativeRotation (Variables|Default|GetMagicCircleScene) (Math|Rotator|MakeRotator _rotaion 0.0 0.0) false false))
            (:Shot
              (Utilities|IsValid (Variables|Default|GetTarget)
                (:Is%20Valid
                  (Game|SpawnActorfromClass "/Game/BluePrints/Effect/Explosion/WaterExplosion/BP_WaterExplosion_v2.BP_WaterExplosion_v2_C" (Math|Transform|MakeTransform (Math|Vector|MakeVector (.x (Transformation|GetActorLocation (Variables|Default|GetTarget))) (.y (Transformation|GetActorLocation (Variables|Default|GetTarget))) 3.0)) "Undefined" 0 0)
                  (Audio|PlaySoundatLocation "/Game/Sound/Magic/Water/SE_WaterExplosion_v1.SE_WaterExplosion_v1" (Math|Vector|MakeVector (.x (Transformation|GetActorLocation (Variables|Default|GetTarget))) (.y (Transformation|GetActorLocation (Variables|Default|GetTarget))) 3.0) "0, 0, 0" 1.0 1.0 0.0 0 0 0))))))))
    (:Is%20Not%20Valid
      (bind _outactors (Actor|GetAllActorswithTag "FireEnemy"))
      (Variables|Default|SetTarget (Utilities|Array|Get(acopy) _outactors))
      (goto _label Reset))))

(fn ConstructionScript)

(fn FNCShot)