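; Water explosion effect actor that chains secondary water explosions and then destroys itself.
; On BeginPlay a timeline stretches the Box component along X by its float track, keeping Y and Z.
; Two timeline event tracks spawn BP_WaterExplosion1 at the Scene and Scene1 transforms, using the root's world scale.
; An older delay-based spawn, collision-toggle and lifespan sequence remains unconnected.
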(event EventBeginPlay
  (bind _scene1 (Variables|Default|GetScene1))
  (bind _box (Variables|Default|GetBox))
  (bind _scene (Variables|Default|GetScene))
  (bind _returnvalue (Transformation|GetSocketTransform _scene1 "None" "RTS_World"))
  (bind _returnvalue_2 (Transformation|GetSocketTransform _scene "None" "RTS_World"))
  (bind _relativescale3d (Variables|/Script/Engine.SceneComponent|GetRelativeScale3D _box))
  (bind _新規track_1 (Timeline|タイムライン_1 PlayFromStart)
    (:Update
      (Transformation|SetRelativeScale3D _box (Math|Vector|MakeVector _新規track_1 (.y _relativescale3d) (.z _relativescale3d))))
    (:Finished
      (Actor|DestroyActor))
    (:新規Track_0
      (Game|SpawnActorfromClass "/Game/BluePrints/Effect/Explosion/WaterExplosion/BP_WaterExplosion1.BP_WaterExplosion1_C" (Math|Transform|MakeTransform (.location _returnvalue_2) (.rotation _returnvalue_2) (Transformation|GetWorldScale (Variables|Default|GetDefaultSceneRoot))) "Undefined" 0 0))
    (:新規Track_2
      (Game|SpawnActorfromClass "/Game/BluePrints/Effect/Explosion/WaterExplosion/BP_WaterExplosion1.BP_WaterExplosion1_C" (Math|Transform|MakeTransform (.location _returnvalue) (.rotation _returnvalue) (Transformation|GetWorldScale (Variables|Default|GetDefaultSceneRoot))) "Undefined" 0 0))))

(fn ConstructionScript)