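; Water slime enemy that takes element-dependent damage from explosions and tracks it on an HP widget.
; Box overlaps read the explosion's actor tag: wind deals high damage, fire middle and water low, via shared damage functions.
; Each hit updates the HP ratio on the widget, hidden at BeginPlay, and calls SetWidgetVisibilty.
; At zero HP or below, the destroy routine matching the explosion's element runs.
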(event OnComponentBeginOverlap(Box)
  (params (OverlappedComponent :type Primitive%20Component%20Object%20Reference) (OtherActor :type Actor%20Object%20Reference) (OtherComp :type Primitive%20Component%20Object%20Reference) (OtherBodyIndex :type Integer) (bFromSweep :type Boolean) (SweepResult :type Hit%20Result%20Structure%20%28by%20ref%29))
  (if (Actor|ActorHasTag OtherActor "FireExplosion")
    (bind _opthp (CallFunction|FncDamageMiddleAttributeExplosion (Variables|Default|GetHP)))
    (bind _output_get (Variables|Default|SetHP _opthp))
    (if (<= _output_get 0.0)
      (CallFunction|UpdHP)
      (CallFunction|FireExplosionDestroy (Variables|Character|GetCharacterMovement) self)
      (else
        (CallFunction|UpdHP)))
    (elif (Actor|ActorHasTag OtherActor "WaterExplosion")
      (bind _opthp_2 (CallFunction|FncDamageLowAttributeExplosion (Variables|Default|GetHP)))
      (bind _output_get_2 (Variables|Default|SetHP _opthp_2))
      (if (<= _output_get_2 0.0)
        (CallFunction|UpdHP)
        (CallFunction|WaterExplosionDestroy (Variables|Character|GetCharacterMovement) self)
        (else
          (CallFunction|UpdHP)))
      (elif (Actor|ActorHasTag OtherActor "WindExplosion")
        (bind _opthp_3 (CallFunction|FncDamageHighAttributeExplosion (Variables|Default|GetHP)))
        (bind _output_get_3 (Variables|Default|SetHP _opthp_3))
        (if (<= _output_get_3 0.0)
          (CallFunction|UpdHP)
          (CallFunction|WindExplosionDestroy (Variables|Character|GetCharacterMovement) self)
          (else
            (CallFunction|UpdHP)))))))

(event Custom|UpdHP
  (Default|UpdateHP (Variables|Default|GetEnemyHPref) (/ (Variables|Default|GetHP) (Variables|Default|GetMaxHP)))
  (CallFunction|SetWidgetVisibilty))

(event EventBeginPlay
  (|CallParentFunction)
  (bind _aswidget_water_enemy_hp (Utilities|Casting|CastToWidget_WaterEnemyHP (UserInterface|GetUserWidgetObject (Variables|Default|GetWidget))))
  (Variables|Default|SetEnemyHPref _aswidget_water_enemy_hp)
  (Rendering|SetVisibility (Variables|Default|GetWidget) false false))

(event Collision|EventActorBeginOverlap
  (params (OtherActor :type Actor%20Object%20Reference))
  (|CallParentFunction OtherActor) ; このノードは無効になっているため呼び出せません。\n機能をビルドするにはピンをドラッグしてください。
)

(fn ConstructionScript
  (|CallParentFunction))