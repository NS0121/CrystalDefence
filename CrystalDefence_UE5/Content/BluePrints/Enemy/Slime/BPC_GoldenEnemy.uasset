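; Golden slime enemy, a child Blueprint with its own HP and a health bar widget that starts hidden.
; Box overlaps with actors tagged as Fire, Water or Wind explosions deal fixed damage, then refresh the bar and its visibility through UpdHP.
; At zero HP it calls the destroy routine matching that explosion's element.
; Tick prints the current HP to screen as debug output.
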(event OnComponentBeginOverlap(Box)
  (params (OverlappedComponent :type Primitive%20Component%20Object%20Reference) (OtherActor :type Actor%20Object%20Reference) (OtherComp :type Primitive%20Component%20Object%20Reference) (OtherBodyIndex :type Integer) (bFromSweep :type Boolean) (SweepResult :type Hit%20Result%20Structure%20%28by%20ref%29))
  (if (Actor|ActorHasTag OtherActor "FireExplosion")
    (bind _output_get (Variables|Default|SetHP (- (Variables|Default|GetHP) 5e+01)))
    (if (<= _output_get 0.0)
      (CallFunction|UpdHP)
      (CallFunction|FireExplosionDestroy (Variables|Character|GetCharacterMovement) self)
      (else
        (CallFunction|UpdHP)))
    (elif (Actor|ActorHasTag OtherActor "WaterExplosion")
      (bind _output_get_2 (Variables|Default|SetHP (- (Variables|Default|GetHP) 5e+01)))
      (if (<= _output_get_2 0.0)
        (CallFunction|UpdHP)
        (CallFunction|WaterExplosionDestroy (Variables|Character|GetCharacterMovement) self)
        (else
          (CallFunction|UpdHP)))
      (elif (Actor|ActorHasTag OtherActor "WindExplosion")
        (bind _output_get_3 (Variables|Default|SetHP (- (Variables|Default|GetHP) 5e+01)))
        (if (<= _output_get_3 0.0)
          (CallFunction|UpdHP)
          (CallFunction|WindExplosionDestroy (Variables|Character|GetCharacterMovement) self)
          (else
            (CallFunction|UpdHP)))))))

(event Custom|UpdHP
  (Default|UpdateHP (Variables|Default|GetEnemyHPref) (/ (Variables|Default|GetHP) (Variables|Default|GetMaxHP)))
  (CallFunction|SetWidgetVisibilty))

(event EventBeginPlay
  (|CallParentFunction)
  (bind _aswidget_golden_enemy_hp (Utilities|Casting|CastToWidget_GoldenEnemyHP (UserInterface|GetUserWidgetObject (Variables|Default|GetWidget))))
  (Variables|Default|SetEnemyHPref _aswidget_golden_enemy_hp)
  (Rendering|SetVisibility (Variables|Default|GetWidget) false false))

(event Collision|EventActorBeginOverlap
  (params (OtherActor :type Actor%20Object%20Reference))
  (|CallParentFunction OtherActor) ; このノードは無効になっているため呼び出せません。\n機能をビルドするにはピンをドラッグしてください。
)

(event EventTick
  (params (DeltaSeconds :type Float%20%28single-precision%29))
  (|CallParentFunction DeltaSeconds)
  (Development|PrintString (Utilities|String|ToString(Float) (Variables|Default|GetHP)) true true "(R=0.000000,G=0.660000,B=1.000000,A=1.000000)" 1.0))

(fn ConstructionScript
  (|CallParentFunction))