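; Base Blueprint for tutorial slime enemies, providing shared death, elemental explosion and damage logic.
; Per-type destroy events stop movement, play the death animation with differing delays, award MP and score, then destroy the actor.
; Helper functions spawn fire, water or wind explosions at the enemy, scaled by charge level.
; Damage functions return new HP per bullet or explosion affinity tier; low-attribute bullets heal instead, capped at max HP.
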(event Custom|Destroy
  (params (CharacterMovement :type Character%20Movement%20Component%20Object%20Reference) (DestroyCharacter :type Character%20Object%20Reference))
  (Variables|/Script/Engine.CharacterMovementComponent|SetMaxWalkSpeed CharacterMovement 0.0)
  (Utilities|FlowControl|Delay 0.0)
  (Components|Animation|PlayAnimation (Variables|Character|GetMesh) "/Game/Models/Slime/NewSlime/slime_death.slime_death" false)
  (bind _asmy_game_instance (Utilities|Casting|CastToMyGameInstance (Game|GetGameInstance)))
  (Default|PlusMP _asmy_game_instance 5.0)
  (Default|PlusScore _asmy_game_instance 1e+01)
  (Utilities|FlowControl|Delay 3.0)
  (Actor|DestroyActor DestroyCharacter))

(event Custom|FireExplosionDestroy
  (params (CharacterMovement :type Character%20Movement%20Component%20Object%20Reference) (DestroyCharacter :type Character%20Object%20Reference))
  (Variables|/Script/Engine.CharacterMovementComponent|SetMaxWalkSpeed CharacterMovement 0.0)
  (Utilities|FlowControl|Delay 0.6)
  (Components|Animation|PlayAnimation (Variables|Character|GetMesh) "/Game/Models/Slime/NewSlime/slime_death.slime_death" false)
  (bind _asmy_game_instance (Utilities|Casting|CastToMyGameInstance (Game|GetGameInstance)))
  (Default|PlusMP _asmy_game_instance 5.0)
  (Default|PlusScore _asmy_game_instance 1e+01)
  (Utilities|FlowControl|Delay 3.0)
  (Actor|DestroyActor DestroyCharacter))

(event Custom|WaterExplosionDestroy
  (params (CharacterMovement :type Character%20Movement%20Component%20Object%20Reference) (DestroyCharacter :type Character%20Object%20Reference))
  (Variables|/Script/Engine.CharacterMovementComponent|SetMaxWalkSpeed CharacterMovement 0.0)
  (Utilities|FlowControl|Delay 1.0)
  (Components|Animation|PlayAnimation (Variables|Character|GetMesh) "/Game/Models/Slime/NewSlime/slime_death.slime_death" false)
  (bind _asmy_game_instance (Utilities|Casting|CastToMyGameInstance (Game|GetGameInstance)))
  (Default|PlusMP _asmy_game_instance 5.0)
  (Default|PlusScore _asmy_game_instance 1e+01)
  (Utilities|FlowControl|Delay 3.0)
  (Actor|DestroyActor DestroyCharacter))

(event Custom|WindExplosionDestroy
  (params (CharacterMovement :type Character%20Movement%20Component%20Object%20Reference) (DestroyCharacter :type Character%20Object%20Reference))
  (Variables|/Script/Engine.CharacterMovementComponent|SetMaxWalkSpeed CharacterMovement 0.0)
  (Components|Animation|PlayAnimation (Variables|Character|GetMesh) 0 false)
  (Utilities|FlowControl|Delay 4.0)
  (Components|Animation|PlayAnimation (Variables|Character|GetMesh) "/Game/Models/Slime/NewSlime/slime_death.slime_death" false)
  (bind _asmy_game_instance (Utilities|Casting|CastToMyGameInstance (Game|GetGameInstance)))
  (Default|PlusMP _asmy_game_instance 5.0)
  (Default|PlusScore _asmy_game_instance 1e+01)
  (Utilities|FlowControl|Delay 3.0)
  (Actor|DestroyActor DestroyCharacter))

(event EventBeginPlay)

(event Collision|EventActorBeginOverlap
  (params (OtherActor :type Actor%20Object%20Reference)))

(event EventTick
  (params (DeltaSeconds :type Float%20%28single-precision%29)))

(fn ConstructionScript)

(fn FncSpawnFireExplosion
  (params (Enemy :type Character%20Object%20Reference) (ChargedLevel :type Float%20%28single-precision%29))
  (bind _returnvalue (Transformation|GetActorLocation Enemy))
  (Game|SpawnActorfromClass "/Game/BluePrints/Effect/Explosion/FireExplosion/BP_FireExplosion.BP_FireExplosion_C" (Math|Transform|MakeTransform (Math|Vector|MakeVector (.x _returnvalue) (.y _returnvalue) (+ (.z _returnvalue) 1.0)) "0, 0, 0" (* "1.000000,1.000000,1.000000" ChargedLevel)) "Undefined" 0 0))

(fn FncSpawnWaterExplosion
  (params (Enemy :type Character%20Object%20Reference) (ChargedLevel :type Float%20%28single-precision%29))
  (bind _returnvalue (Transformation|GetActorLocation Enemy))
  (Game|SpawnActorfromClass "/Game/BluePrints/Effect/Explosion/WaterExplosion/BP_WaterExplosion_v2.BP_WaterExplosion_v2_C" (Math|Transform|MakeTransform (Math|Vector|MakeVector (.x _returnvalue) (.y _returnvalue) (+ (.z _returnvalue) 1.0)) "0, 0, 0" (* "1.000000,1.000000,1.000000" ChargedLevel)) "Undefined" 0 0))

(fn FncSpawnWindExplosion
  (params (Enemy :type Character%20Object%20Reference) (ChargedLevel :type Float%20%28single-precision%29))
  (bind _returnvalue (Transformation|GetActorLocation Enemy))
  (Game|SpawnActorfromClass "/Game/BluePrints/Effect/Explosion/WindExplosion/BP_WindExplosion.BP_WindExplosion_C" (Math|Transform|MakeTransform (Math|Vector|MakeVector (.x _returnvalue) (.y _returnvalue) (+ (.z _returnvalue) 1.0)) "0, 0, 0" (* "1.000000,1.000000,1.000000" ChargedLevel)) "Undefined" 0 0))

(fn FncDamegeNormalBullet
  (params (IptHP :type Float%20%28single-precision%29))
  (bind _normalbullet (Variables|Default|GetNormalBullet))
  (return (- IptHP _normalbullet) _normalbullet))

(fn FncDamageLowAttributeBullet
  (params (IptHP :type Float%20%28single-precision%29) (IptMaxHP :type Float%20%28single-precision%29))
  (bind _lowattributebullet (Variables|Default|GetLowAttributeBullet))
  (bind _returnvalue (+ IptHP _lowattributebullet))
  (if (>= _returnvalue IptMaxHP)
    (return IptMaxHP _lowattributebullet)
    (else
      (return _returnvalue _lowattributebullet))))

(fn FncDamageMiddleAttributeBullet
  (params (IptHP :type Float%20%28single-precision%29))
  (bind _middleattributebullet (Variables|Default|GetMiddleAttributeBullet))
  (return (- IptHP _middleattributebullet) _middleattributebullet))

(fn FncDamageHighAttributeBullet
  (params (IptHP :type Float%20%28single-precision%29))
  (bind _highattributebullet (Variables|Default|GetHighAttributeBullet))
  (return (- IptHP _highattributebullet) _highattributebullet))

(fn FncDamageLowAttributeExplosion
  (params (IptHP :type Float%20%28single-precision%29) (IptMaxHP :type Float%20%28single-precision%29))
  (bind _lowattributeexplosion (Variables|Default|GetLowAttributeExplosion))
  (return (- IptHP _lowattributeexplosion) _lowattributeexplosion))

(fn FncDamageMiddleAttributeExplosion
  (params (IptHP :type Float%20%28single-precision%29))
  (bind _middleattributeexplosion (Variables|Default|GetMiddleAttributeExplosion))
  (return (- IptHP _middleattributeexplosion) _middleattributeexplosion))

(fn FncDamageHighAttributeExplosion
  (params (IptHP :type Float%20%28single-precision%29))
  (bind _highattributeexplosion (Variables|Default|GetHighAttributeExplosion))
  (return (- IptHP _highattributeexplosion) _highattributeexplosion))