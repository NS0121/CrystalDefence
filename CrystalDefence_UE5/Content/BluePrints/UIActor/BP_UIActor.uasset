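; BP_UIActor is a physical menu actor that selects between Tutorial, Normal and Challenge play in what appears to be a VR game.
; It has three collision components, one per mode, whose begin-overlap events only respond to components tagged WandCrystal.
; A matching overlap casts the game mode to VRGameMode and calls its corresponding play function, so touching an option with the wand triggers that mode.
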(event OnComponentBeginOverlap(TutorialCollsiion)
  (params (OverlappedComponent :type Primitive%20Component%20Object%20Reference) (OtherActor :type Actor%20Object%20Reference) (OtherComp :type Primitive%20Component%20Object%20Reference) (OtherBodyIndex :type Integer) (bFromSweep :type Boolean) (SweepResult :type Hit%20Result%20Structure%20%28by%20ref%29))
  (if (Components|ComponentHasTag OtherComp "WandCrystal")
    (bind _asvrgame_mode (Utilities|Casting|CastToVRGameMode (Game|GetGameMode)))
    (Default|FNCTutorialPlay _asvrgame_mode)))

(event OnComponentBeginOverlap(NormalCollision)
  (params (OverlappedComponent :type Primitive%20Component%20Object%20Reference) (OtherActor :type Actor%20Object%20Reference) (OtherComp :type Primitive%20Component%20Object%20Reference) (OtherBodyIndex :type Integer) (bFromSweep :type Boolean) (SweepResult :type Hit%20Result%20Structure%20%28by%20ref%29))
  (if (Components|ComponentHasTag OtherComp "WandCrystal")
    (bind _asvrgame_mode (Utilities|Casting|CastToVRGameMode (Game|GetGameMode)))
    (Default|FNCNormalPlay _asvrgame_mode)))

(event OnComponentBeginOverlap(ChallengeCollision)
  (params (OverlappedComponent :type Primitive%20Component%20Object%20Reference) (OtherActor :type Actor%20Object%20Reference) (OtherComp :type Primitive%20Component%20Object%20Reference) (OtherBodyIndex :type Integer) (bFromSweep :type Boolean) (SweepResult :type Hit%20Result%20Structure%20%28by%20ref%29))
  (if (Components|ComponentHasTag OtherComp "WandCrystal")
    (bind _asvrgame_mode (Utilities|Casting|CastToVRGameMode (Game|GetGameMode)))
    (Default|FNCChallengePlay _asvrgame_mode)))

(event EventBeginPlay)

(event Collision|EventActorBeginOverlap
  (params (OtherActor :type Actor%20Object%20Reference)))

(event EventTick
  (params (DeltaSeconds :type Float%20%28single-precision%29)))

(fn ConstructionScript)