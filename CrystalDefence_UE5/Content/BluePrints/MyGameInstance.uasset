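; Game instance Blueprint that holds MP and score and exposes events to change them.
; PlusMP and MinusMP add or subtract the given amount, clamping MP at MaxMP and MinMP respectively.
; PlusScore increases Score through a plain addition with no limit check.
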(event Custom|PlusMP
  (params (PlusMP :type Float%20%28single-precision%29))
  (bind _maxmp (Variables|Default|GetMaxMP))
  (if (>= (+ PlusMP (Variables|Default|GetMP)) _maxmp)
    (Variables|Default|SetMP _maxmp)
    (else
      (Variables|Default|SetMP (+ PlusMP (Variables|Default|GetMP))))))

(event Custom|MinusMP
  (params (MinusMP :type Float%20%28single-precision%29))
  (bind _minmp (Variables|Default|GetMinMP))
  (if (<= (- (Variables|Default|GetMP) MinusMP) _minmp)
    (Variables|Default|SetMP _minmp)
    (else
      (Variables|Default|SetMP (- (Variables|Default|GetMP) MinusMP)))))

(event Custom|PlusScore
  (params (Score :type Float%20%28single-precision%29))
  (Variables|Default|SetScore (+ Score (Variables|Default|GetScore))))